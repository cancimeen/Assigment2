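; Game instance that shows an on-screen countdown of the seconds left for the Blue team to win.
; CountdownStarter waits briefly, creates the Timer widget, adds it to the viewport and starts Countdown.
; Countdown writes BP_GameState's Countdown value into the widget, waits a second, decrements that value and calls itself again, with no stop condition.
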(event `Countdown Starter`
  (`KismetSystemLibrary.Delay` 2.5)
  (bind _returnvalue (`|CreateWidget` "/Game/Blueprints/UMG/Timer.Timer_C"))
  (bind _output_get (set `self.Count Widget` _returnvalue))
  (`UserWidget.AddToViewport` _output_get 0)
  (`self.Countdown`))

(event `Countdown`
  (bind _countdown (`/Game/Blueprints/BP_GameState.Countdown` (cast `/Game/Blueprints/BP_GameState` (`GameplayStatics.GetGameState`) :!pure true)))
  (`TextBlock.SetText` (`/Game/Blueprints/UMG/Timer.TextBlock_0` (`self.Count Widget`)) (`KismetTextLibrary.Conv_StringToText` (`KismetStringLibrary.Concat_StrStr` (`KismetStringLibrary.Conv_IntToString` _countdown) " Seconds left for Blue team to win ")))
  (`KismetSystemLibrary.Delay` 1.0)
  (`/Engine/EditorBlueprintResources/StandardMacros.DecrementInt` _countdown
    (:`  `
      (`self.Countdown`))))